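; Tank pawn Blueprint that wires player input to C++ aiming and movement components.
; BeginPlay hands the barrel and turret to the aim component and both tracks to the movement component.
; Axis input rotates a gimbal and spring arm for frame-rate-scaled camera aiming, and forwards drive and spin intents to movement.
; Fire calls the aim component, whose projectile class is set in the construction script.
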(event `self.ReceiveBeginPlay`
  ;[1 1 1] Setting the AimComp for c++
  (`AimComponent.AimSetting` (`self.Aim`) (`self.TankBarrel`) (`self.TankTurret`))
  ;[1 1 1] Setting the tracks for C++
  (`TMovementComponent.TrackSetting` (`self.TMovement`) (`self.LeftTrack`) (`self.RightTrack`)))

(event `InputAxis|AimHorizontally`
  (params (AxisValue :type "Float (single-precision)"))
  ;[1 1 1] Horizontal Aiming
  (`SceneComponent.K2_AddLocalRotation` (`self.Horizontal Gimbal`) (`KismetMathLibrary.MakeRotator` 0.0 0.0 (* AxisValue (`GameplayStatics.GetWorldDeltaSeconds`) 100.0)) false false))

(event `InputAxis|Forward`
  (params (AxisValue :type "Float (single-precision)"))
  ;[1 1 1] Movement
  (`TMovementComponent.IntenedMoveForward` (`self.TMovement`) AxisValue))

(event `InputAxis|AimVertical`
  (params (AxisValue :type "Float (single-precision)"))
  ;[1 1 1] Vertical Aiming
  (`SceneComponent.K2_AddLocalRotation` (`self.SpringArm`) (`KismetMathLibrary.MakeRotator` 0.0 (* AxisValue (`GameplayStatics.GetWorldDeltaSeconds`) -100.0)) false false))

(event `InputAxis|SpinClockWise`
  (params (AxisValue :type "Float (single-precision)"))
  ;[1 1 1] Movement
  (`TMovementComponent.IntenedSpinClockWise` (`self.TMovement`) AxisValue))

(event `InputAction|Fire`
  (params (Key :type "Key Structure"))
  (:`Pressed`
    (`AimComponent.Fire` (`self.Aim`))))

(fn `UserConstructionScript`
  (set `AimComponent.ProjectileBlueprint` "/Game/Tank/ProjectileBP.ProjectileBP_C" (`self.Aim`)))